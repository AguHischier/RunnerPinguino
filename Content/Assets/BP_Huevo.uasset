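; BP_Huevo is a collectible pickup (named egg, commented as a coin) that adds one point to the player's score.
; A timeline started on BeginPlay moves the Cube component's relative location, while Tick spins it by a fixed amount each frame, independent of delta time.
; When a ThirdPersonCharacter overlaps the Box, the actor increments that character's Puntuacion and destroys itself.
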(event OnComponentBeginOverlap(Box)
  (params (OverlappedComponent :type Primitive%20Component%20Object%20Reference) (OtherActor :type Actor%20Object%20Reference) (OtherComp :type Primitive%20Component%20Object%20Reference) (OtherBodyIndex :type Integer) (bFromSweep :type Boolean) (SweepResult :type Hit%20Result%20Structure%20%28by%20ref%29))
  ;[1 1 1] Sumar puntos
  (bind _asthird_person_character (Utilities|Casting|CastToThirdPersonCharacter OtherActor))
  (Variables|/Game/ThirdPersonBP/Blueprints/ThirdPersonCharacter.ThirdPersonCharacter_C|SetPuntuacion _asthird_person_character (+ (Variables|/Game/ThirdPersonBP/Blueprints/ThirdPersonCharacter.ThirdPersonCharacter_C|GetPuntuacion _asthird_person_character) 1))
  (Actor|DestroyActor))

(event EventTick
  (params (DeltaSeconds :type Float%20%28single-precision%29))
  ;[1 1 1] Movimiento de la moneda
  (Transformation|AddRelativeRotation (Variables|Default|GetCube) "0,1.000000, 0" false false))

(event EventBeginPlay
  ;[1 1 1] Movimiento de la moneda
  (bind _movimiento (Timeline|MoverMoneda Play)
    (:Update
      (Transformation|SetRelativeLocation (Variables|Default|GetCube) (Math|Vector|MakeVector 0.0 0.0 _movimiento) false false))))

(fn ConstructionScript)