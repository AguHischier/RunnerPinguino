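; Base platform for a runner game that fills itself with random pickups and an optional obstacle on BeginPlay.
; It spawns a few eggs and, rarely, a speed boot at random rotation-relative offsets, storing them in arrays.
; When CrearObstaculo is set, one of three obstacle components becomes visible with overlap collision, and overlapping obstacles kills the ThirdPersonCharacter.
; Delayed cleanup of platform and pickups is disconnected, leaving the Box end-overlap event empty.
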(event OnComponentEndOverlap(Box)
  (params (OverlappedComponent :type Primitive%20Component%20Object%20Reference) (OtherActor :type Actor%20Object%20Reference) (OtherComp :type Primitive%20Component%20Object%20Reference) (OtherBodyIndex :type Integer))
  ;[1 1 1] Destruir objetos y monedas
)

(event OnComponentBeginOverlap(Obstaculo1)
  (params (OverlappedComponent :type Primitive%20Component%20Object%20Reference) (OtherActor :type Actor%20Object%20Reference) (OtherComp :type Primitive%20Component%20Object%20Reference) (OtherBodyIndex :type Integer) (bFromSweep :type Boolean) (SweepResult :type Hit%20Result%20Structure%20%28by%20ref%29))
  ;[1 1 1] Morir  cuando toca un bloque
  (bind _asthird_person_character (Utilities|Casting|CastToThirdPersonCharacter OtherActor))
  (Default|EventoMorir _asthird_person_character))

(event OnComponentBeginOverlap(Obstaculo2)
  (params (OverlappedComponent :type Primitive%20Component%20Object%20Reference) (OtherActor :type Actor%20Object%20Reference) (OtherComp :type Primitive%20Component%20Object%20Reference) (OtherBodyIndex :type Integer) (bFromSweep :type Boolean) (SweepResult :type Hit%20Result%20Structure%20%28by%20ref%29))
  ;[1 1 1] Morir  cuando toca un bloque
  (bind _asthird_person_character (Utilities|Casting|CastToThirdPersonCharacter OtherActor))
  (Default|EventoMorir _asthird_person_character))

(event OnComponentBeginOverlap(Obstaculo3)
  (params (OverlappedComponent :type Primitive%20Component%20Object%20Reference) (OtherActor :type Actor%20Object%20Reference) (OtherComp :type Primitive%20Component%20Object%20Reference) (OtherBodyIndex :type Integer) (bFromSweep :type Boolean) (SweepResult :type Hit%20Result%20Structure%20%28by%20ref%29))
  ;[1 1 1] Morir  cuando toca un bloque
  (bind _asthird_person_character (Utilities|Casting|CastToThirdPersonCharacter OtherActor))
  (Default|EventoMorir _asthird_person_character))

(event Collision|EventActorBeginOverlap
  (params (OtherActor :type Actor%20Object%20Reference)))

(event EventTick
  (params (DeltaSeconds :type Float%20%28single-precision%29)))

(event EventBeginPlay
  (Utilities|FlowControl|Sequence
    (:then_0
      ;[1 1 1] CrearHuevos
      (for _index (range 1 (Math|Random|RandomIntegerinRange 0 2))
        (bind _returnvalue (Game|SpawnActorfromClass "/Game/Assets/BP_Huevo.BP_Huevo_C" (Math|Transform|MakeTransform (+ (Math|Vector|RotateVector (Math|Vector|MakeVector (Math|Random|RandomFloatinRange 4e+01 6e+02) (Math|Random|RandomFloatinRange -2.5e+02 2.5e+02) (Math|Random|RandomFloatinRange 4e+01 1.1e+02)) (Transformation|GetActorRotation)) (Transformation|GetActorLocation)) "0, 0, 0" "1,1,1") "Undefined" 0 0))
        (Utilities|Array|Add (Variables|Default|GetMonedas) _returnvalue)))
    (:then_1
      ;[1 1 1] Crear botas
      (for _index_2 (range 1 (Math|Conversions|ToInteger(Boolean) (<= (Math|Random|RandomIntegerinRange 0 80) 1)))
        (bind _returnvalue_2 (Game|SpawnActorfromClass "/Game/BP_Runner/BP_Velocidad.BP_Velocidad_C" (Math|Transform|MakeTransform (+ (Math|Vector|RotateVector (Math|Vector|MakeVector (Math|Random|RandomFloatinRange 4e+01 6e+02) (Math|Random|RandomFloatinRange -2.5e+02 2.5e+02) (Math|Random|RandomFloatinRange 4e+01 1.1e+02)) (Transformation|GetActorRotation)) (Transformation|GetActorLocation)) "0, 0, 0" "1,1,1") "Undefined" 0 0))
        (Utilities|Array|Add (Variables|Default|GetVelocidad) _returnvalue_2)))
    (:then_2
      ;[1 1 1] Crear obstaculos
      (if (Variables|Default|GetCrearObstaculo)
        (bind _output_get (Variables|Default|SetObstaculoSeleccionado (Utilities|Select :Index (Math|Random|RandomIntegerinRange 0 2) :Option%200 (Variables|Default|GetObstaculo1) :Option%201 (Variables|Default|GetObstaculo2) :Option%202 (Variables|Default|GetObstaculo3))))
        (Rendering|SetVisibility _output_get true false)
        (Collision|SetCollisionProfileName _output_get "OverlapAll" true :!class /Script/Engine.PrimitiveComponent)))))

(fn ConstructionScript)